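; Actor that builds a 3D text string from per-character static meshes in the construction script.
; Fixed row ranges of the DTFont data table fill glyph maps for uppercase, lowercase, digits, symbols and accented letters.
; Each character picks a map by ASCII code, spawns a mesh with the shared material and advances a pivot by glyph width plus spacing.
; Vertical justification sets the starting pivot; horizontal justification shifts all meshes afterwards.
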(event EventBeginPlay)

(event Collision|EventActorBeginOverlap
  (params (OtherActor :type Actor%20Object%20Reference)))

(event EventTick
  (params (DeltaSeconds :type Float%20%28single-precision%29)))

(fn ConstructionScript
  (CallFunction|SetPositionPivot)
  (CallFunction|SetLettersfromDT)
  (for _array_element (Utilities|String|GetCharacterArrayfromString (Variables|Default|GetText))
    (LocalVariables|SetCarTexte _array_element)
    (LocalVariables|SetAsciiLetter (Utilities|String|GetCharacterasNumber _array_element))
    (if (and (>= (LocalVariables|GetAsciiLetter) 65) (<= (LocalVariables|GetAsciiLetter) 90))
      ;[1 1 1] Majuscules
      (CallFunction|AddLetter (LocalVariables|GetCarTexte) (Variables|Default|GetLettersMaj))
      (elif (and (>= (LocalVariables|GetAsciiLetter) 97) (<= (LocalVariables|GetAsciiLetter) 122))
        ;[1 1 1] Miniscules
        (CallFunction|AddLetter (LocalVariables|GetCarTexte) (Variables|Default|GetLettersMin))
        (elif (and (>= (LocalVariables|GetAsciiLetter) 48) (<= (LocalVariables|GetAsciiLetter) 57))
          ;[1 1 1] Chiffres
          (CallFunction|AddLetter (LocalVariables|GetCarTexte) (Variables|Default|GetChiffres))
          (else
            ;[1 1 1] Espace
            (if (== (LocalVariables|GetAsciiLetter) 32)
              (Variables|Default|SetPositionPivot (Math|Vector|MakeVector (+ (.x (Variables|Default|GetPositionPivot)) (Variables|Default|GetEspace)) (.y (Variables|Default|GetPositionPivot)) (.z (Variables|Default|GetPositionPivot))))
              (elif (or (and (>= (LocalVariables|GetAsciiLetter) 33) (<= (LocalVariables|GetAsciiLetter) 47)) (and (>= (LocalVariables|GetAsciiLetter) 58) (<= (LocalVariables|GetAsciiLetter) 64)))
                ;[1 1 1] CaractereSpeciaux
                (CallFunction|AddLetter (LocalVariables|GetCarTexte) (Variables|Default|GetCaractereSpecial))
                (else
                  (CallFunction|AddLetter (LocalVariables|GetCarTexte) (Variables|Default|GetLettresAccentuees))))))))))
  ;[1 1 1] Jusification
  (switch int (Utilities|Array|FindItem (Utilities|Array|MakeArray (Utilities|Enum|Equal(Enum) (Variables|Default|GetJustificationHorizontal) "NewEnumerator1") (Utilities|Enum|Equal(Enum) (Variables|Default|GetJustificationHorizontal) "NewEnumerator0")) true)
    (:0
      (for _array_element_2 (Variables|Default|GetMeshs)
        (Transformation|SetRelativeLocation _array_element_2 (Math|Vector|MakeVector (- (.x (Variables|/Script/Engine.SceneComponent|GetRelativeLocation _array_element_2)) (/ (.x (Variables|Default|GetPositionPivot)) 2.0)) (.y (Variables|/Script/Engine.SceneComponent|GetRelativeLocation _array_element_2)) (.z (Variables|/Script/Engine.SceneComponent|GetRelativeLocation _array_element_2))) false false)))
    (:1
      (for _array_element_3 (Variables|Default|GetMeshs)
        (Transformation|SetRelativeLocation _array_element_3 (Math|Vector|MakeVector (- (.x (Variables|/Script/Engine.SceneComponent|GetRelativeLocation _array_element_3)) (.x (Variables|Default|GetPositionPivot))) (.y (Variables|/Script/Engine.SceneComponent|GetRelativeLocation _array_element_3)) (.z (Variables|/Script/Engine.SceneComponent|GetRelativeLocation _array_element_3))) false false)))))

(fn SetLettersfromDT
  (for _index (range 0 25)
    (bind _returnvalue (Utilities|GetDataTableRow (Variables|Default|GetDT_Font) (Utilities|String|StringToName (Utilities|String|ToString(Integer) _index)))
      (:then
        (Utilities|Map|Add (Variables|Default|GetLettersMaj) (.ID (Utilities|Struct|BreakDataLetters _returnvalue)) (.Lettre (Utilities|Struct|BreakDataLetters _returnvalue))))))
  (for _index_2 (range 26 51)
    (bind _returnvalue_2 (Utilities|GetDataTableRow (Variables|Default|GetDT_Font) (Utilities|String|StringToName (Utilities|String|ToString(Integer) _index_2)))
      (:then
        (Utilities|Map|Add (Variables|Default|GetLettersMin) (.ID (Utilities|Struct|BreakDataLetters _returnvalue_2)) (.Lettre (Utilities|Struct|BreakDataLetters _returnvalue_2))))))
  (for _index_3 (range 53 62)
    (bind _returnvalue_3 (Utilities|GetDataTableRow (Variables|Default|GetDT_Font) (Utilities|String|StringToName (Utilities|String|ToString(Integer) _index_3)))
      (:then
        (Utilities|Map|Add (Variables|Default|GetChiffres) (.ID (Utilities|Struct|BreakDataLetters _returnvalue_3)) (.Lettre (Utilities|Struct|BreakDataLetters _returnvalue_3))))))
  (for _index_4 (range 63 84)
    (bind _returnvalue_4 (Utilities|GetDataTableRow (Variables|Default|GetDT_Font) (Utilities|String|StringToName (Utilities|String|ToString(Integer) _index_4)))
      (:then
        (Utilities|Map|Add (Variables|Default|GetCaractereSpecial) (.ID (Utilities|Struct|BreakDataLetters _returnvalue_4)) (.Lettre (Utilities|Struct|BreakDataLetters _returnvalue_4))))))
  (for _index_5 (range 85 112)
    (bind _returnvalue_5 (Utilities|GetDataTableRow (Variables|Default|GetDT_Font) (Utilities|String|StringToName (Utilities|String|ToString(Integer) _index_5)))
      (:then
        (Utilities|Map|Add (Variables|Default|GetLettresAccentuees) (.ID (Utilities|Struct|BreakDataLetters _returnvalue_5)) (.Lettre (Utilities|Struct|BreakDataLetters _returnvalue_5)))))))

(fn AddLetter
  (params (CarToAdd :type String) (CarTable :type Map%20of%20Strings%20to%20Structs))
  (LocalVariables|SetCarText CarToAdd)
  (if (.ReturnValue (Utilities|Map|Find CarTable (LocalVariables|GetCarText)))
    (bind _returnvalue (AddComponent|AddStaticMeshComponent false (Math|Transform|MakeTransform (Math|Vector|MakeVector (.x (Variables|Default|GetPositionPivot)) (.y (Variables|Default|GetPositionPivot)) (.z (Variables|Default|GetPositionPivot))) "0, 0, 0" "1,1,1")))
    (Components|StaticMesh|SetStaticMesh _returnvalue (.Mesh (Utilities|Struct|BreakLettre (.Value (Utilities|Map|Find CarTable (LocalVariables|GetCarText))))))
    (Rendering|Material|SetMaterial _returnvalue 0 (Variables|Default|GetMaterial))
    (Utilities|Array|Add (Variables|Default|GetMeshs) _returnvalue)
    (Variables|Default|SetPositionPivot (Math|Vector|MakeVector (+ (+ (.Taille (Utilities|Struct|BreakLettre (.Value (Utilities|Map|Find CarTable (LocalVariables|GetCarText))))) (.x (Variables|Default|GetPositionPivot))) (Variables|Default|GetOffset)) (.y (Variables|Default|GetPositionPivot)) (.z (Variables|Default|GetPositionPivot))))))

(fn SetPositionPivot
  (if (Utilities|Enum|Equal(Enum) (Variables|Default|GetJustificationVertical) "NewEnumerator2")
    (Variables|Default|SetPositionPivot "0,52.000000,0.000000")
    (elif (Utilities|Enum|Equal(Enum) (Variables|Default|GetJustificationVertical) "NewEnumerator1")
      (Variables|Default|SetPositionPivot "0,26.000000,0.000000")
      (else
        (Variables|Default|SetPositionPivot "0, 0, 0")))))